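; GameState Blueprint that exposes shared helpers for objectives, resources and player sides.
; A pure sign helper returns -1 for server-sent actions and 1 otherwise, and a color lookup maps a resource index to one of five color variables.
; The objective completion function and the resource RepNotify are empty stubs in this graph.
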(fn ConstructionScript)

(fn OnCompleteObjective
  (params (ObjectiveId :type Integer) (SentByServer :type Boolean)))

(fn GetPlayerModifier
  (params (SentByServer :type Boolean))
  (if SentByServer
    (return -1.0)
    (else
      (return 1.0))))

(fn OnRepRessource)

(fn GetResourceColor
  (params (resourceIndex :type Integer))
  (return (Utilities|Select :Index resourceIndex :Option%200 (Variables|Default|GetResourceColor1) :Option%201 (Variables|Default|GetResourceColor2) :Option%202 (Variables|Default|GetResourceColor3) :Option%203 (Variables|Default|GetResourceColor4) :Option%204 (Variables|Default|GetResourceColor5))))