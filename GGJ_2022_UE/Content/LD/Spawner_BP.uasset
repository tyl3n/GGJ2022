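; Spawner actor that periodically spawns a random tile from its Tiles array at its own location.
; Tick counts down a timer, then calls SpawnTile, rolls a new NextRessourceID and resets the countdown.
; Each frame it feeds timer progress and that ID to its SpawnerHUD_BP widget.
; The displayed ID does not drive the spawn, as SpawnTile makes its own random pick.
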(event EventBeginPlay
  (Variables|Default|SetSpawnTimer (Variables|Default|GetTimeBetweenSpawn))
  (Class|WidgetComponent|SetTickMode (Variables|Default|GetSpawnerTimerHUD) "Enabled"))

(event Collision|EventActorBeginOverlap
  (params (OtherActor :type Actor%20Object%20Reference)))

(event EventTick
  (params (DeltaSeconds :type Float%20%28single-precision%29))
  (bind _output_get (Variables|Default|SetSpawnTimer (- (Variables|Default|GetSpawnTimer) DeltaSeconds)))
  (if (<= _output_get 0.0)
    (CallFunction|SpawnTile)
    (Variables|Default|SetNextRessourceID (Math|Random|RandomInteger 5))
    (Variables|Default|SetSpawnTimer (Variables|Default|GetTimeBetweenSpawn)))
  (bind _asspawner_hud_bp (Utilities|Casting|CastToSpawnerHUD_BP (UserInterface|GetWidget (Variables|Default|GetSpawnerTimerHUD))))
  (Default|UpdateProgress _asspawner_hud_bp (- 1.0 (/ (Variables|Default|GetSpawnTimer) (Variables|Default|GetTimeBetweenSpawn))) (Variables|Default|GetNextRessourceID)))

(fn ConstructionScript)

(fn SpawnTile
  (Game|SpawnActorfromClass (Utilities|Array|Get(acopy) (Variables|Default|GetTiles) (Math|Random|RandomInteger (Utilities|Array|Length (Variables|Default|GetTiles)))) (Math|Conversions|ToTransform(Vector) (Transformation|GetActorLocation)) "Undefined" self 0))