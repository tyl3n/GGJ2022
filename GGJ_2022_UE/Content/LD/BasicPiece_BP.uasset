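; Draggable, mergeable physics piece that takes its color from the owning Spawner_BP's next resource ID via GameState_BP.
; A dynamic material, created on BeginPlay and applied to meshes when they change (box components get hidden), shows merge state: bad placement, highlight, or a timed just-merged effect.
; Tick manually damps the cube's linear and angular velocity with counter-forces and impulses, using separate translation damping while dragged.
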(event Custom|Delay
  (Rendering|Material|SetScalarParameterValue (Variables|Default|GetMaterial) "JustPlaced" 0.0 :!class /Script/Engine.MaterialInstanceDynamic))

(event EventBeginPlay
  (bind _returnvalue (Rendering|Material|CreateDynamicMaterialInstance (Variables|Default|GetCube) 0 "/Game/Material/BoxShader_M.BoxShader_M" "None" :!class /Script/Engine.PrimitiveComponent))
  (bind _output_get (Variables|Default|SetMaterial _returnvalue))
  (bind _asgame_state_bp (Utilities|Casting|CastToGameState_BP (Game|GetGameState)))
  (bind _asspawner_bp (Utilities|Casting|CastToSpawner_BP (Components|GetOwner)))
  (Rendering|Material|SetVectorParameterValue _output_get "Color" (Math|Conversions|ToLinearColor(Color) (Class|GGJGameState|GetResourceColor _asgame_state_bp (Variables|/Game/System/Spawner_BP.Spawner_BP_C|GetNextRessourceID _asspawner_bp))) :!class /Script/Engine.MaterialInstanceDynamic))

(event EventTick
  (params (DeltaSeconds :type Float%20%28single-precision%29))
  (bind _cube (Variables|Default|GetCube))
  (Physics|AddForce _cube (* (* (Transformation|GetComponentVelocity _cube) -1e+02) (Math|Float|Clamp(Float) (* DeltaSeconds (Math|Float|SelectFloat (Variables|Default|GetDraggingTranslationDamping) (Variables|Default|GetTranslationDamping) (Variables|Default|GetbDraging))))) "None" true)
  (Class|PrimitiveComponent|AddAngularImpulseinDegrees _cube (* (* (Physics|GetPhysicsAngularVelocityinDegrees _cube "None") -1.0) (Math|Float|Clamp(Float) (* DeltaSeconds (Variables|Default|GetRotationDamping)))) "None" true))

(event EventOnStaticMeshComponentChanged
  (for _array_element (Variables|Default|GetStaticMeshes)
    (Rendering|Material|SetMaterial _array_element 0 (Variables|Default|GetMaterial))
    (for _array_element_2 (Variables|Default|GetBoxComponents)
      (Development|SetHiddeninGame _array_element_2 true false))))

(event EventOnMergeStateChanged
  (bind _material (Variables|Default|GetMaterial))
  (switch Utilities|FlowControl|Switch|SwitchonEMergeState (Variables|Default|GetMergeState)
    (:None
      (Rendering|Material|SetScalarParameterValue _material "BadPlacement" 0.0 :!class /Script/Engine.MaterialInstanceDynamic)
      (Rendering|Material|SetScalarParameterValue _material "Highlight" 0.0 :!class /Script/Engine.MaterialInstanceDynamic))
    (:OnPadButUnmergable
      (Rendering|Material|SetScalarParameterValue _material "BadPlacement" 1.0 :!class /Script/Engine.MaterialInstanceDynamic)
      (Rendering|Material|SetScalarParameterValue _material "Highlight" 0.0 :!class /Script/Engine.MaterialInstanceDynamic))
    (:OnPadAndMergable
      (Rendering|Material|SetScalarParameterValue _material "Highlight" 1.0 :!class /Script/Engine.MaterialInstanceDynamic)
      (Rendering|Material|SetScalarParameterValue _material "BadPlacement" 0.0 :!class /Script/Engine.MaterialInstanceDynamic))
    (:JustMerged
      (if (Utilities|Time|IsValidTimerHandle (stale _returnvalue))
        (Utilities|Time|ClearandInvalidateTimerbyHandle (stale _returnvalue)))
      (Rendering|Material|SetScalarParameterValue _material "JustPlaced" 1.0 :!class /Script/Engine.MaterialInstanceDynamic)
      (bind _returnvalue (Utilities|Time|SetTimerbyEvent (delegate Custom|Delay) 1.0)))))

(fn ConstructionScript)