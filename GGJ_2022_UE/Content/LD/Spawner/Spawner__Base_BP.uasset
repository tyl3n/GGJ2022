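; Base spawner actor that spawns weighted-random tile pieces on a randomized repeating timer, or once before destroying itself when SingleShot is set.
; Each cycle pre-rolls a weighted resource ID, whose color tints four wall planes through a shared dynamic material.
; Tick feeds countdown progress and that resource to a widget HUD and toggles plane visibility.
; Before spawning, overlapping DraggableActors are pushed outward with force scaled by their mesh count.
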(event EventBeginPlay
  (Variables|Default|SetSpawnTimer (+ (Math|Random|RandomFloatinRange (Variables|Default|GetInitialDelayMin) (Variables|Default|GetInitialDelayMax)) (Variables|Default|GetTimeBetweenSpawn)))
  (Class|WidgetComponent|SetTickMode (Variables|Default|GetSpawnerTimerHUD) "Enabled")
  (bind _resourceid (CallFunction|GetRandomResourceID))
  (bind _output_get (Variables|Default|SetNextRessourceID _resourceid))
  (if (Variables|Default|GetbSingleShot)
    (CallFunction|SpawnTile)
    (Actor|DestroyActor)
    (else
      (Rendering|Material|SetVectorParameterValue (Variables|Default|GetMaterial) "Color" (Math|Conversions|ToLinearColor(Color) (Class|GGJBlueprintLibrary|GetResourceColor 0 _output_get)) :!class /Script/Engine.MaterialInstanceDynamic)
      (bind _asspawner_hud_bp (Utilities|Casting|CastToSpawnerHUD_BP (UserInterface|GetWidget (Variables|Default|GetSpawnerTimerHUD))))
      (Default|UpdateProgress _asspawner_hud_bp (- 1.0 (/ (Variables|Default|GetSpawnTimer) (Variables|Default|GetTimeBetweenSpawn))) (Variables|Default|GetNextRessourceID))
      (Rendering|SetVisibility (Variables|Default|GetPlane3) (> (- 1.0 (/ (Variables|Default|GetSpawnTimer) (Variables|Default|GetTimeBetweenSpawn))) 0.0) false))))

(event EventTick
  (params (DeltaSeconds :type Float%20%28single-precision%29))
  (bind _output_get (Variables|Default|SetSpawnTimer (- (Variables|Default|GetSpawnTimer) DeltaSeconds)))
  (if (<= _output_get 0.0)
    (CallFunction|SpawnTile)
    (Variables|Default|SetSpawnTimer (+ (Math|Random|RandomFloatinRange (Variables|Default|GetSpawnMinRandomDelay) (Variables|Default|GetSpawnMaxRandomDelay)) (Variables|Default|GetTimeBetweenSpawn)))
    (bind _resourceid (CallFunction|GetRandomResourceID))
    (bind _output_get_2 (Variables|Default|SetNextRessourceID _resourceid))
    (if (Variables|Default|GetbSingleShot)
      (CallFunction|SpawnTile)
      (Actor|DestroyActor)
      (else
        (Rendering|Material|SetVectorParameterValue (Variables|Default|GetMaterial) "Color" (Math|Conversions|ToLinearColor(Color) (Class|GGJBlueprintLibrary|GetResourceColor 0 _output_get_2)) :!class /Script/Engine.MaterialInstanceDynamic)
        (bind _asspawner_hud_bp (Utilities|Casting|CastToSpawnerHUD_BP (UserInterface|GetWidget (Variables|Default|GetSpawnerTimerHUD)) :!label _label))
        (Default|UpdateProgress _asspawner_hud_bp (- 1.0 (/ (Variables|Default|GetSpawnTimer) (Variables|Default|GetTimeBetweenSpawn))) (Variables|Default|GetNextRessourceID))
        (Rendering|SetVisibility (Variables|Default|GetPlane3) (> (- 1.0 (/ (Variables|Default|GetSpawnTimer) (Variables|Default|GetTimeBetweenSpawn))) 0.0) false)))
    (else
      (goto _label))))

(fn ConstructionScript
  (bind _resources (Variables|Default|GetResources))
  (bind _returnvalue (Rendering|Material|CreateDynamicMaterialInstance (Variables|Default|GetPlane2) 0 "/Game/Material/SpawnWall_M_Inst.SpawnWall_M_Inst" "None" :!class /Script/Engine.PrimitiveComponent))
  (bind _output_get (Variables|Default|SetMaterial _returnvalue))
  (Rendering|Material|SetMaterial (Variables|Default|GetPlane3) 0 _output_get)
  (if (== (Utilities|Array|Length _resources) 1)
    (Rendering|Material|SetVectorParameterValue (Variables|Default|GetMaterial) "Color" (Math|Conversions|ToLinearColor(Color) (Class|GGJBlueprintLibrary|GetResourceColor self (.resourceid (Utilities|Array|Get(acopy) _resources)))) :!class /Script/Engine.MaterialInstanceDynamic)))

(fn SpawnTile
  (CallFunction|Repulse)
  (bind _piececlass (CallFunction|GetRandomPieceClass))
  (Game|SpawnActorfromClass _piececlass (Math|Conversions|ToTransform(Vector) (Transformation|GetActorLocation)) "AdjustIfPossibleButDontSpawnIfColliding" self 0)
  (Audio|PlaySound2D "/Game/Sound/BRS_Meat_Plop_Small_Squishy.BRS_Meat_Plop_Small_Squishy" 1.0 1.0 0.0 0 0))

(fn GetRandomPieceClass
  (bind _tiles (Variables|Default|GetTiles))
  (for _array_element (Variables|Default|GetTiles)
    (LocalVariables|SetMaxSpawnChance (+ (.chance _array_element) (LocalVariables|GetMaxSpawnChance))))
  (LocalVariables|SetRandomFloat (Math|Random|RandomFloatinRange 0.0 (LocalVariables|GetMaxSpawnChance)))
  (LocalVariables|SetAccumulatedSpawnChance 0.0)
  (for _array_element_2 _tiles
    (if (< (LocalVariables|GetRandomFloat) (+ (.chance _array_element_2) (LocalVariables|GetAccumulatedSpawnChance)))
      (return (.piece _array_element_2))
      (else
        (LocalVariables|SetAccumulatedSpawnChance (+ (.chance _array_element_2) (LocalVariables|GetAccumulatedSpawnChance))))))
  ;[1 1 1] Failsafe
  (return (.piece (Utilities|Array|Get(acopy) _tiles))))

(fn GetRandomResourceID
  (bind _resources (Variables|Default|GetResources))
  (for _array_element (Variables|Default|GetResources)
    (LocalVariables|SetMaxSpawnChance (+ (.chance _array_element) (LocalVariables|GetMaxSpawnChance))))
  (LocalVariables|SetRandomFloat (Math|Random|RandomFloatinRange 0.0 (LocalVariables|GetMaxSpawnChance)))
  (LocalVariables|SetAccumulatedSpawnChance 0.0)
  (for _array_element_2 _resources
    (if (< (LocalVariables|GetRandomFloat) (+ (.chance _array_element_2) (LocalVariables|GetAccumulatedSpawnChance)))
      (return (.resourceid _array_element_2))
      (else
        (LocalVariables|SetAccumulatedSpawnChance (+ (.chance _array_element_2) (LocalVariables|GetAccumulatedSpawnChance))))))
  ;[1 1 1] Failsafe
  (return (.resourceid (Utilities|Array|Get(acopy) _resources))))

(fn Repulse
  (bind _spawnoverlappcollision (Variables|Default|GetSpawnOverlappCollision))
  (bind _returnvalue (Transformation|GetWorldLocation _spawnoverlappcollision))
  (for _array_element (Collision|GetOverlappingActors (Variables|Default|GetSpawnOverlappCollision) "/Script/GGJ_2022_UE.DraggableActor" :!class /Script/Engine.PrimitiveComponent)
    (bind _asdraggable_actor (Utilities|Casting|CastToDraggableActor _array_element))
    (Class|PrimitiveComponent|AddForceatLocation (Variables|/Script/GGJ_2022_UE.DraggableActor|GetMasterStaticMesh _asdraggable_actor) (* (Class|KismetMathLibrary|VectorNormal2D (- (Class|DraggableActor|GetDraggableCenter _asdraggable_actor) _returnvalue) 0.0001) (* (Utilities|Array|Length (Variables|/Script/GGJ_2022_UE.DraggableActor|GetStaticMeshes _asdraggable_actor)) 2.5e+07)) _returnvalue "None")))