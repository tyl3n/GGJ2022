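; Piece Blueprint with a physics Cube and draggable event hooks, apparently a prototype of a movable piece.
; Every Tick it pushes the Cube against its own velocity, acting as velocity-proportional drag.
; The select, drag and release events are empty, and the linear damping calls, one scaled by distance, are disconnected.
; Cube hits print the other actor and component as debug output, except for the actor stored in NewVar0.
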(event OnComponentHit(Cube)
  (params (HitComponent :type Primitive%20Component%20Object%20Reference) (OtherActor :type Actor%20Object%20Reference) (OtherComp :type Primitive%20Component%20Object%20Reference) (NormalImpulse :type Vector :default "0, 0, 0") (Hit :type Hit%20Result%20Structure%20%28by%20ref%29))
  (if (not (== (Variables|Default|GetNewVar_0) OtherActor))
    (Development|PrintString (Utilities|String|ToString(Text) (Utilities|Text|FormatText "{0}.{1}" OtherActor OtherComp)))))

(event EventBeginPlay)

(event Collision|EventActorBeginOverlap
  (params (OtherActor :type Actor%20Object%20Reference)))

(event EventTick
  (params (DeltaSeconds :type Float%20%28single-precision%29))
  (bind _cube (Variables|Default|GetCube))
  (Physics|AddForce _cube (* (Transformation|GetComponentVelocity _cube) -1.0) "None" false))

(event EventOnDragged
  (params (distance :type Float%20%28single-precision%29)))

(event EventOnDraggableReleased)

(event EventOnDraggableSelected)

(fn ConstructionScript)